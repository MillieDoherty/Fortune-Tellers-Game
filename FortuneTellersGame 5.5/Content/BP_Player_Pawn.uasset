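; Player pawn that moves its camera between four preset views: original, bird's eye, crystal ball and wide table.
; LerpCamera plays a whoosh sound, then a timeline eases the camera's relative transform and FOV toward the selected view's camera settings.
; It also sets the player controller's ZoomedOnCrystalBall flag, true only for the crystal ball view during early game states.
; An unconnected demo sequence cycling through views remains in the graph.
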(event `self.ReceiveBeginPlay`)

(event `Lerp Camera`
  (params (`View Position` :type Integer))
  (bind _camera (`self.Camera`))
  (bind _returnvalue (select `int` `View Position` :`0` (`self.OriginalView`) :`1` (`self.BirdsEyeView`) :`2` (`self.CrystalBallView`) :`3` (`self.TableWideView`)))
  ; Camera Lerp
  (bind _asbp_player_controller (cast `/Game/BP_Player_Controller` (`GameplayStatics.GetPlayerController` 0)))
  (if (and (<= (`/Game/BP_Player_Controller.Game_State` _asbp_player_controller) 2) (== `View Position` 2))
    (set `/Game/BP_Player_Controller.ZoomedOnCrystalBall?` true _asbp_player_controller)
    (else
      (set `/Game/BP_Player_Controller.ZoomedOnCrystalBall?` false _asbp_player_controller)))
  (`FMODAudioComponent.Play` (`self.Whoosh`))
  (set `self.CamLerpStartTransform` (`SceneComponent.GetRelativeTransform` _camera))
  (set `self.FOVStart` (`CameraComponent.FieldOfView` _camera))
  (set `self.CamLerpEndTransform` (`SceneComponent.GetRelativeTransform` _returnvalue))
  (set `self.FOVEnd` (`CameraComponent.FieldOfView` _returnvalue))
  (bind (_direction _alpha) (`Timeline|Timeline` :!via `PlayFromStart`)
    (:`Update`
      (bind _result (`|EaseFunction` "EaseInOut" _alpha 0.0 1.0))
      (`SceneComponent.K2_SetRelativeTransform` (`self.Camera`) (`KismetMathLibrary.TLerp` (`self.CamLerpStartTransform`) (`self.CamLerpEndTransform`) _result) true false)
      (`CameraComponent.SetFieldOfView` (`self.Camera`) (`KismetMathLibrary.Lerp` (`self.FOVStart`) (`self.FOVEnd`) _result)))))

(fn `UserConstructionScript`)