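; Player controller that runs a turn-based card and bone-rolling duel, from start screen to win or game-over widgets.
; Right-click steps a four-state round: random enemy threshold, bone spawn, two rerolls, then damage and cleanup.
; Multiplied bone totals meeting the threshold damage the enemy; otherwise the player takes damage, animated on crystal ball and voodoo doll actors.
; Tick polls game start and both health values, while pawn camera lerps follow rounds or Space Bar toggles.
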(event `self.ReceiveBeginPlay`
  ;[0.2837 1 0 0.5] Start Screen
  (bind _returnvalue (`|CreateWidget` "/Game/GUI/WB_Start_Screen.WB_Start_Screen_C" (`GameplayStatics.GetPlayerController` 0)))
  (`UserWidget.AddToViewport` _returnvalue 0)
  (set `self.bShowMouseCursor` true)
  (set `self.bEnableClickEvents` true)
  ;[1 0 0] Event Begin Play - Get Ref to BP Card Spawner (Deck)
  (`self.Lerp Player Camera` 3)
  (bind _outactors (`GameplayStatics.GetAllActorsOfClass` "/Game/BP_Card_Spawner.BP_Card_Spawner_C"))
  (set `self.BP_Spawn_Cards` (`|GetArrayItem` _outactors))
  (bind _outactors_2 (`GameplayStatics.GetAllActorsOfClass` "/Game/Assets/Bones/BP_Bone_Spawner.BP_Bone_Spawner_C"))
  (set `self.BP Bone Spawner` (`|GetArrayItem` _outactors_2))
  (bind _returnvalue_2 (`|CreateWidget` "/Game/GUI/WB_GUI.WB_GUI_C" (`GameplayStatics.GetPlayerController` 0)))
  (`UserWidget.AddToViewport` _returnvalue_2 0)
  (set `self.bShowMouseCursor` true)
  (set `self.bEnableClickEvents` true))

(event `self.ReceiveTick`
  (params (DeltaSeconds :type "Float (single-precision)"))
  ;[1 0 0] Event Tick
  (`self.Start Game Sequence`)
  (`self.Check Player Dead`)
  (`self.Check Enemy Dead`))

(event `Check Player Dead`
  ;[0 1 0.9984 0.5] Check Player Dead
  (if (<= (`self.Player_Health`) 0)
    (`WidgetLayoutLibrary.RemoveAllWidgets`)
    (set `self.bEnableClickEvents` false)
    (bind _returnvalue (`|CreateWidget` "/Game/GUI/WB_Game_Over.WB_Game_Over_C" (`GameplayStatics.GetPlayerController` 0)))
    (`UserWidget.AddToViewport` _returnvalue 0)))

(event `Start Game Sequence`
  ; Start Game Sequence
  (if (`self.StartGame`)
    (`WidgetLayoutLibrary.RemoveAllWidgets`)
    (set `self.GameStarted` true)
    (set `self.StartGame` false)
    (elif (`self.GameStarted`)
      (bind _asbp_player_pawn (cast `/Game/BP_Player_Pawn` (`GameplayStatics.GetPlayerPawn` 0)))
      (bind (_direction _newtrack_1) (`Timeline|Timeline` :!via `PlayFromStart`)
        (:`Update`
          (`self.K2_SetActorTransform` _asbp_player_pawn (`KismetMathLibrary.TLerp` (`self.StartTransform`) (`self.DefaultTransform`) _newtrack_1) false false)
          (`KismetSystemLibrary.Delay` 5.0))))))

(event `Check Cards`
  ;[0.07459 1 0 0.5] Check Bone Numbers and Assign to Array
  (set `self.Bone String` "")
  (`KismetArrayLibrary.Array_Clear` (`self.Bones Array`))
  (bind _outactors (`GameplayStatics.GetAllActorsOfClass` "/Game/Assets/Bones/BP_Bone_Parent.BP_Bone_Parent_C"))
  (for _array_element _outactors
    (`KismetArrayLibrary.Array_Add` (`self.Bones Array`) (`/Game/Assets/Bones/BP_Bone_Parent.Bone_Number` _array_element)))
  ;[1 0 0.8222 0.5] Print Bones to Screen (assign to string for GUI layer to print)
  (for _array_element_2 (`self.Bones Array`)
    (set `self.Bone String` (`KismetStringLibrary.Concat_StrStr` (`self.Bone String`) (`KismetStringLibrary.Conv_IntToString` _array_element_2) ","))))

(event `Check Enemy Dead`
  ;[0 1 0.9984 0.5] Check Enemy Dead
  (if (<= (`self.Enemy_Health`) 0)
    (`WidgetLayoutLibrary.RemoveAllWidgets`)
    (set `self.bEnableClickEvents` false)
    (bind _returnvalue (`|CreateWidget` "/Game/GUI/WB_You_Win.WB_You_Win_C" (`GameplayStatics.GetPlayerController` 0)))
    (`UserWidget.AddToViewport` _returnvalue 0)))

(event `Increment Game State`
  ;[0 0.4967 1] Increment Game State
  (bind _output_get (set `self.Game_State` (+ (`self.Game_State`) 1)))
  (if (> _output_get 3)
    (set `self.Game_State` 0)))

(event `Key|RightMouseButton`
  (params (Key :type "Key Structure"))
  ;[0 0.1347 0.1948 0.5] Alternate, Spawn Cards then Bones
  ;;[0 1 0.9989 0.5] Check if player or enemy dead first
  (:`Pressed`
    (`self.Reset Round Variables`)
    (if (and (> (`self.Player_Health`) 0) (> (`self.Enemy_Health`) 0))
      (switch `int` (`self.Game_State`)
        (:`0`
          ;;[0.3444 1 0 0.5] Draw Hand of Cards + Bones
          (`/Engine/EditorBlueprintResources/StandardMacros.DoOnce` false :!label _label
            (:`Completed`
              (set `/Game/BP_Card_Spawner.Card Counter` 0 (`self.BP_Spawn_Cards`))
              (`self.Lerp Player Camera` 0)
              (`self.New Enemy Attack`)
              (`KismetSystemLibrary.Delay` 2.0)
              (`/Game/Assets/Bones/BP_Bone_Spawner.Spawn Bones` (`self.BP Bone Spawner`))
              (`self.Increment Game State`)
              (`KismetSystemLibrary.Delay` 2.0)
              (`self.Check Cards`)
              (`self.Get Total Bone Score`))))
        (:`1`
          ;;[0.9615 1 0] Re-Roll #1
          (`/Game/Assets/Bones/BP_Bone_Spawner.Spawn Bones` (`self.BP Bone Spawner`))
          (`self.Increment Game State`)
          (`KismetSystemLibrary.Delay` 2.0)
          (`self.Check Cards`)
          (`self.Get Total Bone Score`)
          (goto _label :!via `Reset`))
        (:`2`
          ;;[1 0 0.8077 0.5] Re-Roll #2
          (`/Game/Assets/Bones/BP_Bone_Spawner.Spawn Bones` (`self.BP Bone Spawner`))
          (`self.Increment Game State`)
          (`KismetSystemLibrary.Delay` 2.0)
          (`self.Check Cards`)
          (`self.Get Total Bone Score`))
        (:`3`
          ;;[1 0 0.01109 0.5] Return Cards To Deck After Round / Shuffle
          (`self.Get Total Bone Score`)
          (`KismetSystemLibrary.Delay` 0.6)
          (`self.Evaluate Damage`)
          (`KismetSystemLibrary.Delay` 3.8)
          (`self.Return Cards to Spawner`)
          (`self.Increment Game State`)
          (`self.Destroy All Bones`)
          (`self.Lerp Player Camera` 3)
          (`self.Toggle Crystal Ball Hover`))))))

(event `Get Total Bone Score`
  ;[1 0 0.869 0.5] Get Total Bone Score
  (`KismetSystemLibrary.DelayUntilNextTick`)
  (set `self.Bone Score` 0)
  (bind _outactors (`GameplayStatics.GetAllActorsOfClass` "/Game/Assets/Bones/BP_Bone_Parent.BP_Bone_Parent_C"))
  (for _array_element _outactors
    (set `self.Bone Score` (+ (`self.Bone Score`) (`/Game/Assets/Bones/BP_Bone_Parent.Bone_Number` _array_element))))
  (set `self.Bone Score` (* (`self.Bone Score`) (`self.Ability_Score_Multiplier`)))
  (if (>= (`self.Bone Score`) (`self.Bone Score Threshold`))
    (set `self.ThresholdColour` (make `SlateColor` (struct :`R` 1.0 :`G` 1.0 :`B` 1.0 :`A` 1.0)))
    (else
      (set `self.ThresholdColour` (make `SlateColor` (struct :`R` 0.151042 :`A` 1.0))))))

(event `Return All Bones to Spawner`
  ;[0 0.4967 1] Return Bones to Spawner
  (bind _outactors (`GameplayStatics.GetAllActorsOfClass` "/Game/Assets/Bones/BP_Bone_Parent.BP_Bone_Parent_C"))
  (for _array_element _outactors
    (set `/Game/Assets/Bones/BP_Bone_Parent.Return_To_Spawner` true _array_element)))

(event `Tally Cards and Bones`
  ;[1 0 0.8707 0.5] Tally Cards and Bones
)

(event `Return Cards to Spawner`
  ;[0 0.4967 1] Return Cards to Deck (Spawner)
  (bind _outactors (`GameplayStatics.GetAllActorsOfClass` "/Game/Assets/Cards/BP_Card_Parent.BP_Card_Parent_C"))
  (for _array_element _outactors
    (set `/Game/Assets/Cards/BP_Card_Parent.Draw_Return_Card` false _array_element)))

(event `Reset Round Variables`
  ;[0 0.1347 0.1948 0.5] Alternate, Spawn Cards then Bones
  ;;[1 0 0.2168 0.5] Reset Round Variables (Stops score multipliers carrying over between rounds)
  (set `self.Ability_Score_Multiplier` 1)
  (set `self.BoneTotalColour` (make `SlateColor` (struct :`R` 1.0 :`G` 1.0 :`B` 1.0 :`A` 1.0))))

(event `Set All Bones to Clickable`
  ;[0 0.4967 1] Bones are Clickable
  (bind _outactors (`GameplayStatics.GetAllActorsOfClass` "/Game/Assets/Bones/BP_Bone_Parent.BP_Bone_Parent_C"))
  (for _array_element _outactors
    (set `/Game/Assets/Bones/BP_Bone_Parent.Clickable` true _array_element)))

(event `Set all Bones Not Clickable`
  ;[0 0.4967 1] Set all Bones not clickable
  (bind _outactors (`GameplayStatics.GetAllActorsOfClass` "/Game/Assets/Bones/BP_Bone_Parent.BP_Bone_Parent_C"))
  (for _array_element _outactors
    (set `/Game/Assets/Bones/BP_Bone_Parent.Clickable` false _array_element)))

(event `Redraw Cards`
  ; Redraw Cards
  (`self.Return Cards to Spawner`)
  (set `/Game/BP_Card_Spawner.Card Counter` 0 (`self.BP_Spawn_Cards`)))

(event `New Enemy Attack`
  ; New Enemy Attack Value (Required Bone Threshold & Incoming Damage)
  (set `self.ThresholdColour` (make `SlateColor` (struct :`R` 1.0 :`G` 1.0 :`B` 1.0 :`A` 1.0)))
  (set `self.BoneTotalColour` (make `SlateColor` (struct :`R` 1.0 :`G` 1.0 :`B` 1.0 :`A` 1.0)))
  (set `self.Bone Score Threshold` (`KismetMathLibrary.RandomIntegerInRange` 15 45))
  (if (>= (`self.Bone Score Threshold`) 25)
    (if (>= (`self.Bone Score Threshold`) 38)
      (set `self.Threshold Fail Damage` 1)
      (else
        (set `self.Threshold Fail Damage` 2)))
    (else
      (set `self.Threshold Fail Damage` 3))))

(event `Destroy All Bones`
  ;[1 0.1129 0 0.5] Destroy All Bones
  (bind _outactors (`GameplayStatics.GetAllActorsOfClass` "/Game/Assets/Bones/BP_Bone_Parent.BP_Bone_Parent_C"))
  (for _array_element _outactors
    (`self.K2_DestroyActor` _array_element)))

(event `Evaluate Damage`
  ; Evaluate Damage (End of Turn)
  (set `self.ZoomedOnCrystalBall?` false)
  (`self.Toggle Crystal Ball Hover`)
  (bind _asbp_player_pawn (cast `/Game/BP_Player_Pawn` (`GameplayStatics.GetPlayerPawn` 0)))
  (`/Game/BP_Player_Pawn.Lerp Camera` _asbp_player_pawn 2)
  (if (>= (`self.Bone Score`) (`self.Bone Score Threshold`))
    (`self.Enemy Takes Damage` 1)
    (else
      (`self.Player Takes Damage` (`self.Threshold Fail Damage`)))))

(event `Player Takes Damage`
  (params (Damage :type Integer))
  ; Player Takes Damage
  (set `self.Player_Health` (- (`self.Player_Health`) Damage))
  (`KismetSystemLibrary.Delay` 1.0)
  (bind _outactors (`GameplayStatics.GetAllActorsOfClass` "/Game/Assets/VoodooDoll/BP_VoodooDoll.BP_VoodooDoll_C"))
  (for _array_element _outactors
    (`self.Lerp Player Camera` 3)
    (`/Game/Assets/VoodooDoll/BP_VoodooDoll.DamageAnimation` _array_element (`self.Player_Health`))))

(event `Player Heals Damage`
  (params (`Health Gained` :type Integer))
  (bind _output_get (set `self.Player_Health` (+ `Health Gained` (`self.Player_Health`))))
  (if (> _output_get 6)
    (set `self.Player_Health` 6))
  (`KismetSystemLibrary.Delay` 0.3)
  (bind _outactors (`GameplayStatics.GetAllActorsOfClass` "/Game/Assets/VoodooDoll/BP_VoodooDoll.BP_VoodooDoll_C"))
  (for _array_element _outactors
    (`self.Lerp Player Camera` 3)
    (`/Game/Assets/VoodooDoll/BP_VoodooDoll.Heal Animation` _array_element (`self.Player_Health`))))

(event `Enemy Takes Damage`
  (params (Damage :type Integer))
  ; Enemy Takes Damage
  (set `self.Enemy_Health` (- (`self.Enemy_Health`) Damage))
  (`KismetSystemLibrary.Delay` 1.0)
  (bind _outactors (`GameplayStatics.GetAllActorsOfClass` "/Game/Assets/Crystal_Ball/BP_Crystal_Ball.BP_Crystal_Ball_C"))
  (for _array_element _outactors
    (`/Game/Assets/Crystal_Ball/BP_Crystal_Ball.DamageAnimation` _array_element)))

(event `Revert Cam`
  (if (and (<= (`self.Game_State`) 2) (not (`self.CamLerpDisabled`))) :!label _label_2
    (bind _asbp_player_pawn (cast `/Game/BP_Player_Pawn` (`GameplayStatics.GetPlayerPawn` 0)))
    (`/Engine/EditorBlueprintResources/StandardMacros.FlipFlop`
      (:`A`
        (`/Game/BP_Player_Pawn.Lerp Camera` _asbp_player_pawn 1))
      (:`B`
        (`/Game/BP_Player_Pawn.Lerp Camera` _asbp_player_pawn 0)))))

(event `Key|SpaceBar`
  (params (Key :type "Key Structure"))
  (:`Pressed`
    (goto _label_2)))

(event `Lerp Player Camera`
  (params (`Camera View` :type Integer))
  (bind _asbp_player_pawn (cast `/Game/BP_Player_Pawn` (`GameplayStatics.GetPlayerPawn` 0)))
  (`/Game/BP_Player_Pawn.Lerp Camera` _asbp_player_pawn `Camera View`))

(event `Toggle Crystal Ball Hover`
  (bind _outactors (`GameplayStatics.GetAllActorsOfClass` "/Game/Assets/Crystal_Ball/BP_Crystal_Ball.BP_Crystal_Ball_C"))
  (for _array_element _outactors
    (if (`/Game/Assets/Crystal_Ball/BP_Crystal_Ball.HoverDisabled?` _array_element)
      (set `/Game/Assets/Crystal_Ball/BP_Crystal_Ball.HoverDisabled?` false _array_element)
      (set `self.CamLerpDisabled` false)
      (else
        (set `/Game/Assets/Crystal_Ball/BP_Crystal_Ball.HoverDisabled?` true _array_element)
        (set `self.CamLerpDisabled` true)))))

(fn `UserConstructionScript`)