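; Dialogue handler for the fortune teller card game that shows spoken lines for drawn tarot cards through the player controller's GameCardText.
; The Dialogue event picks a random line from the card's array, queuing the following entry for two hard-coded two-part lines.
; A timer fires AdvanceDialogue to clear or advance the text, with DoOnce gates controlling re-entry.
; Intro and round or game outcome branches are empty.
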(event `Dialogue`
  (params (CardDraw :type Boolean) (`Card Number` :type Integer) (Intro :type Boolean) (WinRound :type Boolean) (LoseRound :type Boolean) (WinGame :type Boolean) (LoseGame :type Boolean))
  (bind _returnvalue (select `int` (+ `Card Number` -1) :`0` (`self.DialogueTheHermit`) :`1` (`self.DialogueTheFool`) :`2` (`self.DialogueTheLovers`) :`3` (`self.DialogueTheMoon`) :`4` (`self.DialogueTheMagician`) :`5` (`self.DialogueTheHangedMan`) :`6` (`self.DialogueTheChariot`) :`7` (`self.DialogueTheSun`) :`8` (`self.DialogueTheDeath`) :`9` (`self.DialogueTheHighPriestess`)))
  (if CardDraw
    (set `self.IsNextLine?` 0)
    (bind _output_get (set `self.CurrentLine` (`|GetArrayItem` _returnvalue (`KismetMathLibrary.RandomIntegerInRange` 0 2))))
    (switch `string` _output_get
      (:`Default`
        _)
      (:`A crossroads of a million paths but a single life…`
        (set `self.IsNextLine?` 1 :!label _label)
        (set `self.NextLine` (`|GetArrayItem` _returnvalue (+ (`KismetArrayLibrary.Array_Find` _returnvalue (`self.CurrentLine`)) 1))))
      (:`My child, embrace neither code nor creed of the universe,`
        (goto _label)))
    ;[0 0.1989 1 0.5] Hover Over Card (Start)
    (`/Engine/EditorBlueprintResources/StandardMacros.DoOnce` false :!label _label_2
      (:`Completed`
        (bind _asbp_player_controller (cast `/Game/BP_Player_Controller` (`GameplayStatics.GetPlayerController` 0)))
        (set `/Game/BP_Player_Controller.Game_Card_Text` (`self.CurrentLine`) _asbp_player_controller)
        (`KismetSystemLibrary.K2_SetTimerDelegate` (delegate `Advance Dialogue`) 3.0)
        (set `self.CanProgressDialogue?` true)
        (goto _label_3 :!via `Reset`)))
    (elif Intro
      _
      (elif WinRound
        _
        (elif LoseRound
          _
          (elif WinGame
            _
            (elif LoseGame
              _)))))))

(event `Advance Dialogue`
  ;[0 0.1989 1 0.5] Hover Over Card (End)
  (`/Engine/EditorBlueprintResources/StandardMacros.DoOnce` false :!label _label_3
    (:`Completed`
      (bind _asbp_player_controller (cast `/Game/BP_Player_Controller` (`GameplayStatics.GetPlayerController` 0)))
      (set `/Game/BP_Player_Controller.Game_Card_Text` "" _asbp_player_controller)
      (if (== (`self.IsNextLine?`) 1)
        (set `/Game/BP_Player_Controller.Game_Card_Text` (`self.NextLine`) (stale `Dialogue` _asbp_player_controller))
        (set `self.CanProgressDialogue?` false)
        (`KismetSystemLibrary.Delay` 0.2)
        (set `self.CanProgressDialogue?` true)
        (set `self.IsNextLine?` 0)
        (goto _label_3 :!via `Reset`)
        (else
          (goto _label_2 :!via `Reset`))))))

(event `Key|LeftMouseButton`
  (params (Key :type "Key Structure")))

(fn `UserConstructionScript`)