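; Fortune teller actor that idly turns back and forth around the yaw it has at BeginPlay.
; Each Tick eases the current yaw a small fraction toward a target yaw, leaving pitch and roll unchanged.
; A Delay in the Tick chain picks a new target every few seconds at random, as a small random offset from the original yaw.
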(event `self.ReceiveBeginPlay`
  (bind (_returnvalue_roll _returnvalue_pitch _returnvalue_yaw) (`KismetMathLibrary.BreakRotator` (`self.K2_GetActorRotation`)))
  (bind _output_get (set `self.Z Rotation Original` _returnvalue_yaw))
  (set `self.new rotation` _output_get))

(event `self.ReceiveTick`
  (params (DeltaSeconds :type "Float (single-precision)"))
  (bind (_returnvalue_roll _returnvalue_pitch _returnvalue_yaw) (`KismetMathLibrary.BreakRotator` (`self.K2_GetActorRotation`)))
  ; Comment
  (`self.K2_SetActorRotation` (`KismetMathLibrary.MakeRotator` _returnvalue_roll _returnvalue_pitch (`KismetMathLibrary.FInterpEaseInOut` _returnvalue_yaw (`self.new rotation`) 0.05 1.0)))
  (`KismetSystemLibrary.Delay` (`KismetMathLibrary.RandomFloatInRange` 1.0 5.0))
  (set `self.new rotation` (+ (`self.Z Rotation Original`) (`KismetMathLibrary.RandomFloatInRange` -5.0 5.0))))

(fn `UserConstructionScript`)