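; The Moon card, number 4, a child card Blueprint that boosts the player's ability score multiplier when activated.
; BeginPlay sets its description, which reads "Double damage", and its number.
; ActivateEffect adds one to AbilityScoreMultiplier on BP_Player_Controller rather than doubling it, then destroys the card.
; Tick only calls the parent.
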(event `self.ReceiveBeginPlay`
  (`parent.ReceiveBeginPlay`)
  (set `self.Card Description` "The Moon: Double damage")
  (set `self.Card Number` 4))

(event `self.ReceiveTick`
  (params (DeltaSeconds :type "Float (single-precision)"))
  ;[0 0.6383 1 0.5] Execute Action for Moon
  (`parent.ReceiveTick` DeltaSeconds))

(event `self.Activate Effect`
  ;[0.9868 0 1 0.5] Ability - Increment score Multiplier
  (`KismetSystemLibrary.PrintString` "Moon Card Activated")
  (bind _asbp_player_controller (cast `/Game/BP_Player_Controller` (`GameplayStatics.GetPlayerController` 0)))
  (set `/Game/BP_Player_Controller.Ability_Score_Multiplier` (+ (`/Game/BP_Player_Controller.Ability_Score_Multiplier` _asbp_player_controller) 1) _asbp_player_controller)
  (`self.K2_DestroyActor`))

(fn `UserConstructionScript`
  (`parent.UserConstructionScript`))