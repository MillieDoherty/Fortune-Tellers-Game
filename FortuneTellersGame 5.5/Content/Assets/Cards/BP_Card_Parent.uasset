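; BP_Card_Parent is a base card actor that travels between deck and table, reacts to mouse hover and highlights when active.
; Tick drives a timeline lerp to CardDestination or, when DrawReturnCard is false, a lerp back to its spawn transform before destruction.
; A cursor trace on the capsule toggles an eased lift, plays a sound and sends the description to BP_Player_Controller.
; When flagged, it shows its outline if the controller's BonesArray contains CardNumber.
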(event `Card Hovering`
  (bind _returnvalue (`SceneComponent.K2_GetComponentToWorld` (`self.Scene`)))
  ;[1 0.797 0 0.5] Card Hovering
  (if (`self.Hovering`)
    (set `self.Hovering_Offset` 5.0)
    (else
      (set `self.Hovering_Offset` 0.0)))
  (bind _output_get (set `self.Hovering_Lerp_State` (`KismetMathLibrary.Lerp` (`self.Hovering_Lerp_State`) (`self.Hovering_Offset`) 0.25)))
  (`SceneComponent.K2_SetWorldTransform` (`self.Card_Plane`) (`KismetMathLibrary.MakeTransform` (`KismetMathLibrary.MakeVector` (.x (.location _returnvalue)) (.y (.location _returnvalue)) (+ _output_get (.z (.location _returnvalue)))) (.rotation _returnvalue) (.scale _returnvalue)) false false))

(event `self.ReceiveTick`
  (params (DeltaSeconds :type "Float (single-precision)"))
  ;[1 0 0.01457 0.5] Event Tick
  (`self.Check Cards Active`)
  (`self.Mouse Over Check` 0.0)
  (`self.Card Hovering`)
  (if (`self.Draw_Return_Card`)
    (`self.Move Card To Table`)
    (else
      (`self.Return Card to Deck`))))

(event `self.ReceiveBeginPlay`
  (bind (_returnvalue_roll _returnvalue_pitch) (`KismetMathLibrary.BreakRotator` (`SceneComponent.K2_GetComponentRotation` (`self.Scene`))))
  ;[0 0.927 1 0.5] Start Rotated so it swirls
  (`SceneComponent.K2_SetWorldRotation` (`self.Scene`) (`KismetMathLibrary.MakeRotator` _returnvalue_roll _returnvalue_pitch 180.0) false false)
  (set `self.Origin` (`SceneComponent.K2_GetComponentToWorld` (`self.Scene`))))

(event `Move Card To Table`
  ;[0.1601 1 0] Move towards card point on Table
  (`TimelineComponent.SetPlayRate` (`self.Move Card Timeline`) 0.25)
  (bind (_direction _move_track) (`Timeline|Move Card Timeline`)
    (:`Update`
      (`SceneComponent.K2_SetWorldTransform` (`self.Scene`) (`KismetMathLibrary.TLerp` (`SceneComponent.K2_GetComponentToWorld` (`self.Scene`)) (`self.Card Destination`) _move_track) false false)
      (if (== (`SceneComponent.K2_GetComponentToWorld` (`self.Scene`)) (`self.Card Destination`))
        _))))

(event `Return Card to Deck`
  ;[0.1601 1 0] Return Card to Deck
  (`SceneComponent.K2_SetWorldTransform` (`self.Scene`) (`KismetMathLibrary.TLerp` (`SceneComponent.K2_GetComponentToWorld` (`self.Scene`)) (`self.Origin`) 0.05) false false)
  (`KismetSystemLibrary.Delay` 0.4)
  (`self.K2_DestroyActor`))

(event `Mouse Over Check`
  (params (DeltaSeconds :type "Float (single-precision)"))
  ;[0 0.1989 1 0.5] Card Hover Event
  (if (== (`self.Capsule`) (`.HitComponent` (`GameplayStatics.BreakHitResult` (`PlayerController.GetHitResultUnderCursorByChannel` (`GameplayStatics.GetPlayerController` 0) "TraceTypeQuery1" true))))
    ;[0 0.1989 1 0.5] Hover Over Card (Start)
    (`/Engine/EditorBlueprintResources/StandardMacros.DoOnce` false :!label _label
      (:`Completed`
        (set `self.Hovering` true)
        (`FMODAudioComponent.Play` (`self.HoverSFX`))
        (bind _asbp_player_controller (cast `/Game/BP_Player_Controller` (`GameplayStatics.GetPlayerController` 0)))
        (set `/Game/BP_Player_Controller.Game_Card_Text` (`self.Card Description`) _asbp_player_controller)
        (goto _label_2 :!via `Reset`)))
    (else
      ;[0 0.1989 1 0.5] Hover Over Card (End)
      (`/Engine/EditorBlueprintResources/StandardMacros.DoOnce` false :!label _label_2
        (:`Completed`
          (set `self.Hovering` false)
          (bind _asbp_player_controller_2 (cast `/Game/BP_Player_Controller` (`GameplayStatics.GetPlayerController` 0)))
          (set `/Game/BP_Player_Controller.Game_Card_Text` "" _asbp_player_controller_2)
          (goto _label :!via `Reset`))))))

(event `Check Cards Active`
  ;[1 0 0.06983 0.5] Check if Bone # == Card # Then Highlight
  (if (`self.Check_Card_Num_Activated`)
    (bind _asbp_player_controller (cast `/Game/BP_Player_Controller` (`GameplayStatics.GetPlayerController` 0)))
    (if (`KismetArrayLibrary.Array_Contains` (`/Game/BP_Player_Controller.Bones Array` _asbp_player_controller) (`self.Card Number`))
      (set `self.Card Activated` true)
      (`SceneComponent.SetVisibility` (`self.CardOutline`) true false)
      (else
        (set `self.Card Activated` false)
        (`SceneComponent.SetVisibility` (`self.CardOutline`) false false)))
    (set `self.Check_Card_Num_Activated` false)))

(fn `UserConstructionScript`)