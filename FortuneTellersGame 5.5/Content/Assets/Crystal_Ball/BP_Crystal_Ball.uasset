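; Interactive crystal ball actor that displays enemy health through six flames and serves as a camera zoom target.
; Tick traces under the cursor, using paired DoOnce gates to toggle an outline overlay and play a hover sound.
; Clicking rattles the ball and zooms the player controller's camera, or reverts it if already zoomed.
; Damage plays timeline-driven shake, glass particles and camera shake before updating flames, while healing updates them immediately.
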(event `Start CrystalBall`
  ; Wiggles the Ball in an attempt to fix the texture pop-in issue, doesn't work though
)

(event `self.ReceiveTick`
  (params (DeltaSeconds :type "Float (single-precision)"))
  (if (and (== self (`.HitActor` (`GameplayStatics.BreakHitResult` (`PlayerController.GetHitResultUnderCursorByChannel` (`GameplayStatics.GetPlayerController` 0) "TraceTypeQuery1" true)))) (not (`self.HoverDisabled?`)))
    (`/Engine/EditorBlueprintResources/StandardMacros.DoOnce` false :!label _label
      (:`Completed`
        (`MeshComponent.SetOverlayMaterial` (`self.StaticMesh1`) "/Game/Assets/Effects/MA_OutlineOverlay.MA_OutlineOverlay")
        (`FMODAudioComponent.Play` (`self.Whoosh`))
        (set `self.IsMouseHovering?` true)
        (goto _label_2 :!via `Reset`)))
    (else
      ; Hover Over (End)
      (`/Engine/EditorBlueprintResources/StandardMacros.DoOnce` false :!label _label_2
        (:`Completed`
          (`MeshComponent.SetOverlayMaterial` (`self.StaticMesh1`) null)
          (set `self.IsMouseHovering?` false)
          (goto _label :!via `Reset`))))))

(event `self.ReceiveBeginPlay`
  (set `self.FlamesArray` (`|MakeArray` (`self.Flame6`) (`self.Flame5`) (`self.Flame4`) (`self.Flame3`) (`self.Flame2`) (`self.Flame1`)))
  ; Crystal Ball Zoom Camera On Click
  (add `self.OnClicked` (delegate `OnClicked_Event`)))

(event `OnClicked_Event` :!signature `self.OnClicked`
  (params (TouchedActor :type "Actor Object Reference") (ButtonPressed :type "Key Structure" :default "None"))
  ; Crystal Ball Zoom Camera On Click
  (bind _asbp_player_controller (cast `/Game/BP_Player_Controller` (`GameplayStatics.GetPlayerController` 0)))
  (if (`/Game/BP_Player_Controller.ZoomedOnCrystalBall?` _asbp_player_controller)
    (`/Game/BP_Player_Controller.Revert Cam` _asbp_player_controller)
    (elif (`self.IsMouseHovering?`)
      (`FMODAudioComponent.Play` (`self.CrystalRattle`))
      (`self.RattleAnimation`)
      (`/Game/BP_Player_Controller.Lerp Player Camera` _asbp_player_controller 2))))

(event `RattleAnimation`
  (bind (_default_rotation_roll _default_rotation_pitch _default_rotation_yaw) (`KismetMathLibrary.BreakRotator` (`self.Default Rotation`)))
  (bind (_direction _newtrack_0) (`Timeline|Rattle` :!via `PlayFromStart`)
    (:`Update`
      (`self.K2_SetActorRotation` (`KismetMathLibrary.MakeRotator` (+ (`KismetMathLibrary.MapRangeClamped` _newtrack_0 -1.0 1.0 -10.0 10.0) _default_rotation_roll) _default_rotation_pitch _default_rotation_yaw)))))

(event `DamageAnimation`
  (params (`Enemy Health` :type Integer))
  (bind _staticmesh (`self.StaticMesh`))
  (bind (_relativelocation_x _relativelocation_y) (`KismetMathLibrary.BreakVector` (`SceneComponent.RelativeLocation` _staticmesh)))
  (`TimelineComponent.SetPlayRate` (`self.GlassBreak`) 0.75)
  (`FMODAudioComponent.Play` (`self.CrystalDamage`))
  (bind (_direction _newtrack_0) (`Timeline|GlassBreak` :!via `ReverseFromEnd`)
    (:`Update`
      (bind _returnvalue (+ (`KismetMathLibrary.MapRangeClamped` _newtrack_0 -1.0 1.0 -0.3 0.3) 0.0))
      (`SceneComponent.K2_SetRelativeLocation` _staticmesh (`KismetMathLibrary.MakeVector` _returnvalue _relativelocation_y _returnvalue) false false))
    (:`Finished`
      (`self.RattleAnimation`)
      (`ActorComponent.Activate` (`self.GlassBreakParticles`) false)
      (`GameplayStatics.PlayWorldCameraShake` "/Game/Assets/Effects/BP_CamShakeMedium.BP_CamShakeMedium_C" (`self.K2_GetActorLocation`) 0.0 500.0)
      (`self.Update Flames` `Enemy Health`))))

(event `Heal Animation`
  (params (`Enemy Health` :type Integer))
  (`self.Update Flames` `Enemy Health`))

(event `Update Flames`
  (params (`Enemy Health` :type Integer))
  (for (_array_element _array_index) (`self.FlamesArray`)
    (if (> (+ _array_index 1) `Enemy Health`)
      (`ActorComponent.Deactivate` _array_element)
      (else
        (`ActorComponent.Activate` _array_element false)))))

(fn `UserConstructionScript`)