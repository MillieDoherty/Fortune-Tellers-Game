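; BP_TheLovers_Heal is a child Blueprint that heals the player when destroyed while activated.
; On BeginPlay it sets the ButtonStaticMesh reference to its Cube component, and Tick defers to the parent class.
; On Destroyed it spawns tiny smoke-puff and spark Niagara effects at its location.
; If Activated is set, it then calls PlayerHealsDamage on player 0's BP_Player_Controller to heal one point.
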(event `self.ReceiveBeginPlay`
  (set `self.ButtonStaticMesh` (`self.Cube`)))

(event `self.ReceiveTick`
  (params (DeltaSeconds :type "Float (single-precision)"))
  (`parent.ReceiveTick` DeltaSeconds))

(event `self.ReceiveDestroyed`
  (bind _returnvalue (`self.K2_GetActorLocation`))
  (`NiagaraFunctionLibrary.SpawnSystemAtLocation` "/Game/Assets/Effects/NI_SmokePuff.NI_SmokePuff" _returnvalue (struct) (0.01 0.01 0.01))
  (`NiagaraFunctionLibrary.SpawnSystemAtLocation` "/Game/Assets/Effects/NI_Sparks.NI_Sparks" _returnvalue (struct) (0.01 0.01 0.01))
  (if (`self.Activated`)
    (bind _asbp_player_controller (cast `/Game/BP_Player_Controller` (`GameplayStatics.GetPlayerController` 0)))
    (`/Game/BP_Player_Controller.Player Heals Damage` _asbp_player_controller 1)))

(fn `UserConstructionScript`)