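; BP_Breakable_Button is a clickable button actor that highlights under the cursor and disappears when clicked.
; Tick compares the cursor trace hit with the button mesh, using paired DoOnce gates to toggle an outline overlay and play a click sound once per hover.
; Clicking the Cube sets Activated, spawns point sounds, plays a camera shake, then destroys itself and any valid PairedButton.
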(event `self.ReceiveBeginPlay`)

(event `self.ReceiveTick`
  (params (DeltaSeconds :type "Float (single-precision)"))
  ; Hover Over Bone (Start)
  (if (and (== (`self.ButtonStaticMesh`) (`.HitComponent` (`GameplayStatics.BreakHitResult` (`PlayerController.GetHitResultUnderCursorByChannel` (`GameplayStatics.GetPlayerController` 0) "TraceTypeQuery1" true)))) (`KismetSystemLibrary.IsValid` (`self.ButtonStaticMesh`)))
    (`/Engine/EditorBlueprintResources/StandardMacros.DoOnce` false :!label _label
      (:`Completed`
        (`MeshComponent.SetOverlayMaterial` (`self.ButtonStaticMesh`) "/Game/Assets/Effects/MA_OutlineOverlay.MA_OutlineOverlay")
        (`FMODAudioComponent.Play` (`self.BoneClick`))
        (goto _label_2 :!via `Reset`)))
    (else
      ; Hover Over Bone (End)
      (`/Engine/EditorBlueprintResources/StandardMacros.DoOnce` false :!label _label_2
        (:`Completed`
          (`MeshComponent.SetOverlayMaterial` (`self.ButtonStaticMesh`) null)
          (goto _label :!via `Reset`))))))

(event `self.Cube.OnClicked`
  (params (TouchedComponent :type "PrimitiveComponent Object Reference") (ButtonPressed :type "Key Structure"))
  (bind _pairedbutton (`self.PairedButton`))
  (set `self.Activated` true)
  (`|SpawnActorFromClass` "/Game/Assets/FMOD/BP_PointSound.BP_PointSound_C" (`self.GetTransform`) "AlwaysSpawn" "MultiplyWithRoot" null 0.0 "/Game/FMOD/Events/BoneClickPoof.BoneClickPoof" null)
  (`|SpawnActorFromClass` "/Game/Assets/FMOD/BP_PointSound.BP_PointSound_C" (`self.GetTransform`) "AlwaysSpawn" "MultiplyWithRoot" null 0.0 "/Game/FMOD/Events/BoneClick.BoneClick" null)
  (`GameplayStatics.PlayWorldCameraShake` "/Game/Assets/Effects/BP_CamShakeSmall.BP_CamShakeSmall_C" (`self.K2_GetActorLocation`) 0.0 500.0)
  (`/Engine/EditorBlueprintResources/StandardMacros.IsValid` _pairedbutton
    (:`Is Valid`
      (`self.K2_DestroyActor` _pairedbutton))
    (:`Is Not Valid`
      _))
  (`self.K2_DestroyActor`))

(fn `UserConstructionScript`)