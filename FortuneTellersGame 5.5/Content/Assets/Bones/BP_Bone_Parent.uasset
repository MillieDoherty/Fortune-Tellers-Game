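; BP_Bone_Parent is the base bone actor, which lands on a table with impact effects and can be returned toward its spawner.
; Its first hit on a TableSurface actor plays sounds, sparks and a camera shake, and activates the owning BP_Bone_Spawner's SparkRing.
; While ReturnToSpawner is set, Tick restarts a timeline that lerps the Bone toward a hardcoded point, then destroys the actor after a delay with smoke and sparks.
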(event `self.ReceiveTick`
  (params (DeltaSeconds :type "Float (single-precision)"))
  ;[1 0 0.7576 0.5] Return Bones
  ;; Easier to Convert to Event
  (if (`self.Return_To_Spawner`)
    (`TimelineComponent.SetPlayRate` (`self.Move Target Timeline`) 1.0)
    (bind (_direction _move_track) (`Timeline|Move Target Timeline` :!via `PlayFromStart`)
      (:`Update`
        (`SceneComponent.K2_SetWorldLocation` (`self.Bone`) (`KismetMathLibrary.VLerp` (`self.K2_GetActorLocation`) (0.0 0.0 200.0) _move_track) false false)
        (`KismetSystemLibrary.Delay` 2.0)
        (`self.K2_DestroyActor`)))))

(event `self.ReceiveHit`
  (params (MyComp :type "PrimitiveComponent Object Reference") (Other :type "Actor Object Reference") (OtherComp :type "PrimitiveComponent Object Reference") (bSelfMoved :type Boolean) (HitLocation :type "Vector Structure") (HitNormal :type "Vector Structure") (NormalImpulse :type "Vector Structure") (Hit :type "HitResult Structure (by ref)"))
  (bind _returnvalue (`self.K2_GetActorLocation`))
  ; When Land On Table
  (if (`self.ActorHasTag` Other "TableSurface")
    (`/Engine/EditorBlueprintResources/StandardMacros.DoOnce` false
      (:`Completed`
        (`FMODAudioComponent.Play` (`self.BoneThump`))
        (`FMODAudioComponent.Play` (`self.BoneSpark`))
        (`NiagaraFunctionLibrary.SpawnSystemAtLocation` "/Game/Assets/Effects/NI_Sparks.NI_Sparks" _returnvalue (struct) (0.01 0.01 0.01))
        (`GameplayStatics.PlayWorldCameraShake` "/Game/Assets/Effects/BP_CamShakeSmall.BP_CamShakeSmall_C" _returnvalue 0.0 500.0)
        (bind _asbp_bone_spawner (cast `/Game/Assets/Bones/BP_Bone_Spawner` (`self.GetOwner`)))
        (`ActorComponent.Activate` (`/Game/Assets/Bones/BP_Bone_Spawner.SparkRing` _asbp_bone_spawner) false)))))

(event `self.ReceiveDestroyed`
  (bind _returnvalue (`self.K2_GetActorLocation`))
  ; Particles When Destroyed
  (`NiagaraFunctionLibrary.SpawnSystemAtLocation` "/Game/Assets/Effects/NI_SmokePuff.NI_SmokePuff" _returnvalue (struct) (0.01 0.01 0.01))
  (`NiagaraFunctionLibrary.SpawnSystemAtLocation` "/Game/Assets/Effects/NI_Sparks.NI_Sparks" _returnvalue (struct) (0.01 0.01 0.01)))

(fn `UserConstructionScript`)