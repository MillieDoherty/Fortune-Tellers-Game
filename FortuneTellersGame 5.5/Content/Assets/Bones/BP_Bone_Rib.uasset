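; BP_Bone_Rib is a clickable rib bone actor that plays a throw sound when it spawns.
; Each tick, a cursor trace checks its capsule, with paired DoOnce gates toggling an outline overlay, playing a hover sound and printing the bone number.
; Clicking the capsule spawns two point-sound actors for click and poof, plays a small world camera shake, then destroys the bone.
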(event `self.ReceiveBeginPlay`
  ; SFX Throw (Rattle)
  (`/Engine/EditorBlueprintResources/StandardMacros.DoOnce` false
    (:`Completed`
      (cast `/Game/BP_Player_Controller` (`GameplayStatics.GetPlayerController` 0))
      (`FMODAudioComponent.Play` (`self.BoneThrowSFX`)))))

(event `self.Capsule.OnClicked`
  (params (TouchedComponent :type "PrimitiveComponent Object Reference") (ButtonPressed :type "Key Structure"))
  ; SFX Throw (Thud)
  (`|SpawnActorFromClass` "/Game/Assets/FMOD/BP_PointSound.BP_PointSound_C" (`self.GetTransform`) "AlwaysSpawn" "MultiplyWithRoot" null 0.0 "/Game/FMOD/Events/BoneClickPoof.BoneClickPoof" null)
  (`|SpawnActorFromClass` "/Game/Assets/FMOD/BP_PointSound.BP_PointSound_C" (`self.GetTransform`) "AlwaysSpawn" "MultiplyWithRoot" null 0.0 "/Game/FMOD/Events/BoneClick.BoneClick" null)
  (`GameplayStatics.PlayWorldCameraShake` "/Game/Assets/Effects/BP_CamShakeSmall.BP_CamShakeSmall_C" (`self.K2_GetActorLocation`) 0.0 500.0)
  (`self.K2_DestroyActor`))

(event `self.ReceiveTick`
  (params (DeltaSeconds :type "Float (single-precision)"))
  ; Hover Over Bone (Start)
  (if (== (`self.Capsule`) (`.HitComponent` (`GameplayStatics.BreakHitResult` (`PlayerController.GetHitResultUnderCursorByChannel` (`GameplayStatics.GetPlayerController` 0) "TraceTypeQuery1" true))))
    (`/Engine/EditorBlueprintResources/StandardMacros.DoOnce` false :!label _label
      (:`Completed`
        (`MeshComponent.SetOverlayMaterial` (`self.Bone`) "/Game/Assets/Effects/MA_OutlineOverlay.MA_OutlineOverlay")
        (`FMODAudioComponent.Play` (`self.BoneClick`))
        (`KismetSystemLibrary.PrintString` (`KismetStringLibrary.Conv_IntToString` (`self.Bone_Number`)))
        (goto _label_2 :!via `Reset`)))
    (else
      ; Hover Over Bone (End)
      (`/Engine/EditorBlueprintResources/StandardMacros.DoOnce` false :!label _label_2
        (:`Completed`
          (`MeshComponent.SetOverlayMaterial` (`self.Bone`) null)
          (goto _label :!via `Reset`))))))

(fn `UserConstructionScript`
  (`parent.UserConstructionScript`))