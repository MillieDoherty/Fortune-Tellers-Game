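; BP_Bone_Spawner is an actor that throws bones for a roll, topping the level up to five bones.
; SpawnBones counts existing BP_Bone_Parent actors and spawns a BP_Bone_Rib for each one missing.
; Each rib takes a random pick from eleven spawn points with a random yaw, and stores that point's one-based index as BoneNumber.
; Picked points stay in the pool, so bones can share one.
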(event `Spawn Bones`
  (bind _returnvalue (`SceneComponent.K2_GetComponentToWorld` (`self.CurrentBoneSpawnPoint`)))
  ;[0 0.4124 1 0.5] Throw Bones
  (set `self.Bones Spawnpoints` (`|MakeArray` (`self.Spawn_Point_1`) (`self.Spawn_Point_2`) (`self.Spawn_Point_3`) (`self.Spawn_Point_4`) (`self.Spawn_Point_5`) (`self.Spawn_Point_6`) (`self.Spawn_Point_7`) (`self.Spawn_Point_8`) (`self.Spawn_Point_9`) (`self.Spawn_Point_10`) (`self.Spawn_Point_11`)))
  (bind _outactors (`GameplayStatics.GetAllActorsOfClass` "/Game/Assets/Bones/BP_Bone_Parent.BP_Bone_Parent_C"))
  (for _ (range (+ (- 4 (`KismetArrayLibrary.Array_Length` _outactors)) 1))
    (bind _output_get (set `self.CurrentBoneSpawnPoint` (`KismetArrayLibrary.Array_Random` (`self.Bones Spawnpoints`))))
    (bind _returnvalue_2 (`|SpawnActorFromClass` "/Game/Assets/Bones/BP_Bone_Rib.BP_Bone_Rib_C" (`KismetMathLibrary.MakeTransform` (.location _returnvalue) (`KismetMathLibrary.MakeRotator` (.roll (.rotation _returnvalue)) (.pitch (.rotation _returnvalue)) (`KismetMathLibrary.RandomFloatInRange` 0.0 360.0)) (.scale _returnvalue)) "Undefined" "MultiplyWithRoot" self null))
    (set `/Game/Assets/Bones/BP_Bone_Parent.Bone_Number` (+ (`KismetArrayLibrary.Array_Find` (`self.Bones Spawnpoints`) _output_get) 1) _returnvalue_2)))

(fn `UserConstructionScript`)