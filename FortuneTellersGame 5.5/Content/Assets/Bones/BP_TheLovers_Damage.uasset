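; Damage half of The Lovers pair, a button actor that deals damage to the enemy when destroyed.
; On BeginPlay it spawns BP_TheLovers_Heal slightly offset along X, with each actor set as the other's owner.
; On destruction it plays smoke and spark Niagara effects, calls EnemyTakesDamage on the player controller, then destroys its owner, removing the Heal counterpart.
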(event `self.ReceiveBeginPlay`
  (bind _returnvalue (`self.GetTransform`))
  (set `self.ButtonStaticMesh` (`self.Cube`))
  (bind _returnvalue_2 (`|SpawnActorFromClass` "/Game/Assets/Bones/BP_TheLovers_Heal.BP_TheLovers_Heal_C" (`KismetMathLibrary.MakeTransform` (`KismetMathLibrary.MakeVector` (+ (.x (.location _returnvalue)) 10.0) (.y (.location _returnvalue)) (.z (.location _returnvalue))) (.rotation _returnvalue) (.scale _returnvalue)) "Undefined" "MultiplyWithRoot" self null))
  (`self.SetOwner` _returnvalue_2))

(event `self.ReceiveDestroyed`
  (bind _returnvalue (`self.K2_GetActorLocation`))
  (`NiagaraFunctionLibrary.SpawnSystemAtLocation` "/Game/Assets/Effects/NI_SmokePuff.NI_SmokePuff" _returnvalue (struct) (0.01 0.01 0.01))
  (`NiagaraFunctionLibrary.SpawnSystemAtLocation` "/Game/Assets/Effects/NI_Sparks.NI_Sparks" _returnvalue (struct) (0.01 0.01 0.01))
  (bind _asbp_player_controller (cast `/Game/BP_Player_Controller` (`GameplayStatics.GetPlayerController` 0)))
  (`/Game/BP_Player_Controller.Enemy Takes Damage` _asbp_player_controller 1)
  (`self.K2_DestroyActor` (`self.GetOwner`)))

(fn `UserConstructionScript`)