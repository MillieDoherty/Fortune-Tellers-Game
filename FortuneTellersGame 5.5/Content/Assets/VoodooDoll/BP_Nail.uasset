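; BP_Nail is the voodoo doll's nail actor, which animates a stab into the doll when StabDoll is called.
; It shows the mesh, then two chained timelines ease the actor between stored transforms: rest to above the doll, then down into the stab.
; An event track in the second timeline hides the nail, and completion teleports it back to rest.
; The event's Health input is unused.
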(event `Stab Doll`
  (params (Health :type Integer))
  (`SceneComponent.SetVisibility` (`self.REPLACE_Nail`) true false)
  (bind (_direction _alpha) (`Timeline|Timeline` :!via `PlayFromStart`)
    (:`Update`
      (`self.K2_SetActorTransform` (`KismetMathLibrary.TLerp` (`self.Default Transform`) (`self.Above Doll Transform`) (`KismetMathLibrary.FInterpEaseInOut` 0.0 1.0 _alpha 2.0)) true))
    (:`Finished`
      (bind (_direction_2 _alpha_2) (`Timeline|Timeline_0` :!via `PlayFromStart`)
        (:`Update`
          (`self.K2_SetActorTransform` (`KismetMathLibrary.TLerp` (`self.Above Doll Transform`) (`self.Stab Doll Transform`) (`KismetMathLibrary.FInterpEaseInOut` 0.0 1.0 _alpha_2 2.0)) true))
        (:`Finished`
          (`self.K2_SetActorTransform` (`self.Default Transform`) false true))
        (:`Invisible`
          (`SceneComponent.SetVisibility` (`self.REPLACE_Nail`) false false))))))

(fn `UserConstructionScript`)