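; Voodoo doll actor that plays a damage sequence and displays lost health as pins stuck in the doll.
; DamageAnimation passes health to every BP_Nail, then chained timelines ease the doll to screen centre, shake it and ease it back.
; Timed camera shakes, a Damage playback and a Niagara blood burst punctuate the hits.
; UpdateNails reveals up to six pins by swapping material slots on the doll mesh according to DollHealth.
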(event `DamageAnimation`
  (params (Health :type Integer))
  (bind _outactors (`GameplayStatics.GetAllActorsOfClass` "/Game/Assets/VoodooDoll/BP_Nail.BP_Nail_C"))
  (for _array_element _outactors
    (`/Game/Assets/VoodooDoll/BP_Nail.Stab Doll` _array_element Health)
    (set `self.DollHealth` Health)
    (bind (_direction _alpha) (`Timeline|Timeline` :!via `PlayFromStart`)
      (:`Update`
        (`self.K2_SetActorTransform` (`KismetMathLibrary.TLerp` (`self.DefaultTransform`) (`self.CentreOfScreen`) (`|EaseFunction` "EaseInOut" _alpha 0.0 1.0)) true))
      (:`Finished`
        (`FMODAudioComponent.Play` (`self.Damage`))
        (`GameplayStatics.PlayWorldCameraShake` "/Game/Assets/Effects/BP_CamShakeSmall.BP_CamShakeSmall_C" (`self.K2_GetActorLocation`) 0.0 500.0)
        (bind (_direction_2 _newtrack_0) (`Timeline|Timeline_0` :!via `ReverseFromEnd`)
          (:`Update`
            (bind _returnvalue (`KismetMathLibrary.MapRangeClamped` _newtrack_0 -1.0 1.0 -0.3 0.3))
            (`SceneComponent.K2_SetRelativeLocation` (`self.VoodooDoll`) (`KismetMathLibrary.MakeVector` _returnvalue 0.0 _returnvalue) false false))
          (:`Finished`
            (`KismetSystemLibrary.Delay` 0.5)
            (`GameplayStatics.PlayWorldCameraShake` "/Game/Assets/Effects/BP_CamShakeSmall.BP_CamShakeSmall_C" (`self.K2_GetActorLocation`) 0.0 500.0)
            (bind (_direction_3 _newtrack_0_2) (`Timeline|Timeline_1` :!via `PlayFromStart`)
              (:`Update`
                (`SceneComponent.K2_SetRelativeLocation` (`self.VoodooDoll`) (`KismetMathLibrary.MakeVector` 0.0 (`KismetMathLibrary.MapRangeClamped` _newtrack_0_2 -1.0 1.0 -0.3 0.3)) false false))
              (:`Finished`
                (`KismetSystemLibrary.Delay` 0.3)
                (`GameplayStatics.PlayWorldCameraShake` "/Game/Assets/Effects/BP_CamShakeSmall.BP_CamShakeSmall_C" (`self.K2_GetActorLocation`) 0.0 500.0)
                (`KismetSystemLibrary.Delay` 0.37)
                (`GameplayStatics.PlayWorldCameraShake` "/Game/Assets/Effects/BP_CamShakeMedium.BP_CamShakeMedium_C" (`self.K2_GetActorLocation`) 0.0 500.0)
                (`ActorComponent.Activate` (`self.NI_Blood`) false)
                (`self.Update Nails`)
                (bind (_direction_4 _newtrack_0_3) (`Timeline|Timeline_2` :!via `PlayFromStart`)
                  (:`Update`
                    (bind _returnvalue_2 (`KismetMathLibrary.MapRangeClamped` _newtrack_0_3 -1.0 1.0 -0.3 0.3))
                    (`SceneComponent.K2_SetRelativeLocation` (`self.VoodooDoll`) (`KismetMathLibrary.MakeVector` _returnvalue_2 0.0 _returnvalue_2) false false))
                  (:`Finished`
                    (bind (_direction_5 _alpha_2) (`Timeline|Timeline_3` :!via `ReverseFromEnd`)
                      (:`Update`
                        (`self.K2_SetActorTransform` (`KismetMathLibrary.TLerp` (`self.DefaultTransform`) (`self.CentreOfScreen`) (`|EaseFunction` "EaseInOut" _alpha_2 0.0 1.0)) true)))))))))))))

(event `Update Nails`
  (for _index (range (+ (- 5 (`self.DollHealth`)) 1))
    (bind _returnvalue (select `int` _index :`0` (`self.Nail1 MatIndex`) :`1` (`self.Nail2 MatIndex`) :`2` (`self.Nail3 MatIndex`) :`3` (`self.Nail4 MatIndex`) :`4` (`self.Nail5 MatIndex`) :`5` (`self.Nail6 MatIndex`)))
    (`PrimitiveComponent.SetMaterial` (`self.VoodooDoll`) _returnvalue "/Game/Assets/VoodooDoll/M_PinHead.M_PinHead")
    (`PrimitiveComponent.SetMaterial` (`self.VoodooDoll`) (+ _returnvalue 1) "/Game/Assets/VoodooDoll/M_Pin.M_Pin")))

(event `self.ReceiveBeginPlay`)

(fn `UserConstructionScript`)