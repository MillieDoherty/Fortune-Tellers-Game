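; BP_Card_Spawner is an actor that shuffles a card deck on BeginPlay and deals three cards.
; Tick calls SpawnCard, where a short Delay paces each spawn just above the Cube component, with audio.
; Each BP_Card_Parent card receives a destination transform from Cube1, Cube2 or Cube3, selected by CardCounter.
; Once three cards are out, the counter is never reset, so the deck reshuffles every tick.
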(event `SpawnCard`
  (bind _returnvalue (`SceneComponent.K2_GetComponentToWorld` (`self.Cube`)))
  (bind (_returnvalue_location _returnvalue_rotation) (`KismetMathLibrary.BreakTransform` (`SceneComponent.K2_GetComponentToWorld` (select `int` (`self.Card Counter`) :`0` (`self.Cube1`) :`1` (`self.Cube2`) :`2` (`self.Cube3`)))))
  ;[0 1 0.01143 0.5] Spawn Cards and Shuffle if necessary
  (if (<= (`self.Card Counter`) 2)
    (`KismetSystemLibrary.Delay` 0.25)
    (bind _returnvalue_2 (`|SpawnActorFromClass` (`|GetArrayItem` (`self.Card_Deck`) (`self.Card Counter`)) (`KismetMathLibrary.MakeTransform` (`KismetMathLibrary.MakeVector` (.x (.location _returnvalue)) (.y (.location _returnvalue)) (+ (.z (.location _returnvalue)) 10.0))) "AlwaysSpawn" "MultiplyWithRoot" null null))
    (bind _asbp_card_parent (cast `/Game/Assets/Cards/BP_Card_Parent` _returnvalue_2))
    (set `/Game/Assets/Cards/BP_Card_Parent.Card Destination` (`KismetMathLibrary.MakeTransform` _returnvalue_location _returnvalue_rotation) _asbp_card_parent)
    (`FMODAudioComponent.Play` (`self.CardSpawnAudio`))
    (set `self.Card Counter` (+ (`self.Card Counter`) 1))
    (else
      (`self.Shuffle Cards`))))

(event `self.ReceiveBeginPlay`
  ;[1 0 0] Event Begin Play
  (`self.Shuffle Cards`))

(event `self.ReceiveTick`
  (params (DeltaSeconds :type "Float (single-precision)"))
  ;[1 0 0] Event Tick
  (`self.SpawnCard`))

(event `Shuffle Cards`
  ;[0.1761 0 1 0.5] Shuffle Deck
  (`KismetArrayLibrary.Array_Shuffle` (`self.Card_Deck`)))

(fn `UserConstructionScript`)